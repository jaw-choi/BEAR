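; BP_Door is a two-panel sliding door that opens when something overlaps its Box trigger.
; The first overlap plays a sliding sound and runs a timeline that lerps RightSide and LeftSide apart along Y.
; Ending an overlap reverses the timeline to close the panels.
; A DoOnce with no reset wired limits the opening and sound to a single trigger.
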(event OnComponentBeginOverlap(Box)
  (params (OverlappedComponent :type Primitive%20Component%20Object%20Reference) (OtherActor :type Actor%20Object%20Reference) (OtherComp :type Primitive%20Component%20Object%20Reference) (OtherBodyIndex :type Integer) (bFromSweep :type Boolean) (SweepResult :type Hit%20Result%20Structure%20%28by%20ref%29))
  (Utilities|FlowControl|DoOnce false
    (:Completed
      (Audio|PlaySound2D "/Game/Assets/SFX/slidingDoorCue.slidingDoorCue" 1.0 1.0 0.0 0 0)
      (bind _doormovement (Timeline|Timeline_0 Play)
        (:Update
          (Utilities|FlowControl|Sequence
            (:then_0
              (Transformation|SetRelativeLocation (Variables|Default|GetRightSide) (Math|Vector|Lerp(Vector) "0, 0, 0" "0,200.000000, 0" _doormovement) false false))
            (:then_1
              (Transformation|SetRelativeLocation (Variables|Default|GetLeftSide) (Math|Vector|Lerp(Vector) "0,-200.000000, 0" "0,-400.000000, 0" _doormovement) false false))))))))

(event OnComponentEndOverlap(Box)
  (params (OverlappedComponent :type Primitive%20Component%20Object%20Reference) (OtherActor :type Actor%20Object%20Reference) (OtherComp :type Primitive%20Component%20Object%20Reference) (OtherBodyIndex :type Integer))
  (bind _doormovement (Timeline|Timeline_0 Reverse)
    (:Update
      (Utilities|FlowControl|Sequence
        (:then_0
          (Transformation|SetRelativeLocation (Variables|Default|GetRightSide) (Math|Vector|Lerp(Vector) "0, 0, 0" "0,200.000000, 0" _doormovement) false false))
        (:then_1
          (Transformation|SetRelativeLocation (Variables|Default|GetLeftSide) (Math|Vector|Lerp(Vector) "0,-200.000000, 0" "0,-400.000000, 0" _doormovement) false false))))))

(fn ConstructionScript)