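; Enemy drone pawn that patrols placed points, chases the player on sight and reloads the current level upon catching them.
; Two looping timers replace Tick: one runs player detection, the other drives FloatingPawnMovement by flying mode (Patrolling, Aggro, Looking for Player).
; Detection combines a dot-product view cone with a line trace, ignoring ragdolled players.
; Losing sight enters a search state, which spins at the last-seen location before resuming patrol.
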(event Custom|LFPMovement
  (if (> (Math|Vector|VectorLength (- (Transformation|GetActorLocation) (Variables|Aggro|GetLast%20Saw%20Player%20Location))) (Variables|Default|GetAggro%20Acceptance%20Radius))
    (CallFunction|DoMovementTick true true (Variables|Aggro|GetLast%20Saw%20Player%20Location))
    (else
      (Variables|/Script/Engine.MovementComponent|SetVelocity (Variables|Default|GetFloatingPawnMovement) "0, 0, 0")
      (bind _result (Math|Integer|IncrementInt (Variables|Default|GetLooking%20For%20Player%20Counter))
        (:%20%20
          (if (> _result (Variables|Default|GetMaxLFP))
            (Variables|Movement|SetFlyingMode "NewEnumerator0")
            (else
              (Class|Actor|AddActorWorldRotation (Math|Rotator|MakeRotator 0.0 0.0 (Math|Float|SafeDivide 3.6e+02 (Math|Conversions|ToFloat(Integer) (Variables|Default|GetMaxLFP))))))))))))

(event Custom|CheckForPlayer
  ;[1 1 1] Check for Player
  (bind (_location _foundplayer_) (CallFunction|TraceforPlayer))
  (if _foundplayer_
    (Variables|Aggro|SetLast%20Saw%20Player%20Location _location)
    (Variables|Movement|SetFlyingMode "NewEnumerator1")
    (else
      (switch Utilities|FlowControl|Switch|SwitchonE_DRONE_MODE (Variables|Movement|GetFlyingMode)
        (:NewEnumerator1
          (Variables|Movement|SetFlyingMode "NewEnumerator2")
          (Variables|Default|SetLooking%20For%20Player%20Counter 0))))))

(event Custom|MovementTic
  ;[1 1 1] Movement Tick
  (switch Utilities|FlowControl|Switch|SwitchonE_DRONE_MODE (Variables|Movement|GetFlyingMode)
    (:NewEnumerator0
      (CallFunction|PatrolMovement))
    (:NewEnumerator1
      (CallFunction|AggroMovement))
    (:NewEnumerator2
      (CallFunction|LFPMovement))))

(event Custom|DoMovementTick
  (params (DoForwardMovement :type Boolean) (DoRotation :type Boolean) (Location :type Vector))
  (bind _returnvalue (Transformation|GetActorForwardVector))
  ;[1 1 1] Movement
  (Utilities|FlowControl|Sequence
    (:then_0
      (if DoRotation
        (Transformation|SetActorRotation (Math|Interpolation|RInterpTo (Transformation|GetActorRotation) (Math|Conversions|RotationFromXVector (Math|Vector|Normalize (- Location (Transformation|GetActorLocation)))) (Variables|Movement|GetMovementTickRate) (Utilities|Select :Index (Variables|Movement|GetFlyingMode) :NewEnumerator0 (Variables|Patrol|GetPatrolRinterpSpeed) :NewEnumerator1 (Variables|Aggro|GetAggroRInterpSpeed) :NewEnumerator2 0.0)))))
    (:then_1
      (if DoForwardMovement
        (Class|PawnMovementComponent|AddInputVector (Variables|Default|GetFloatingPawnMovement) (* (Math|Vector|MakeVector (.x _returnvalue) (.y _returnvalue) (.z _returnvalue)) (Utilities|Select :Index (Variables|Movement|GetFlyingMode) :NewEnumerator0 (Variables|Patrol|GetPatrolMoveSpeed) :NewEnumerator1 (Variables|Aggro|GetAggroMoveSpeed) :NewEnumerator2 0.0)) false)))))

(event Custom|AggroMovement
  (if true
    (bind _returnvalue (AddComponent|AddAudioComponent false))
    (Variables|Default|SetDrone%20Detecting%20Player _returnvalue)
    (if (> (Math|Vector|VectorLength (- (Transformation|GetActorLocation) (Variables|Aggro|GetLast%20Saw%20Player%20Location))) (Variables|Default|GetAggro%20Acceptance%20Radius))
      (CallFunction|DoMovementTick true true (Variables|Aggro|GetLast%20Saw%20Player%20Location))
      (else
        (bind _returnvalue_2 (Audio|CreateSound2D "/Game/Assets/SFX/droneCatchingCue.droneCatchingCue" 1.0 1.0 0.0 0 true))
        (bind _output_get (Variables|Default|SetDrone%20Catching%20Player _returnvalue_2))
        (Audio|Components|Audio|Play _output_get 0.0)
        (bind _returnvalue_3 (Game|GetCurrentLevelName true))
        (Game|OpenLevel(byName) (Utilities|String|StringToName _returnvalue_3))
        (CallFunction|DoMovementTick false true (Variables|Aggro|GetLast%20Saw%20Player%20Location))
        (Variables|/Script/Engine.MovementComponent|SetVelocity (Variables|Default|GetFloatingPawnMovement) "0, 0, 0")))
    (else
      (Audio|Components|Audio|Stop (Variables|Default|GetDrone%20Detecting%20Player)))))

(event Custom|PatrolMovement
  (bind _patrolpoints (Variables|Patrol|GetPatrolPoints))
  (bind _patrolindex (Variables|Patrol|GetPatrolIndex))
  (bind _output (Utilities|Array|Get(acopy) _patrolpoints _patrolindex))
  ;[1 1 1] Patrol
  (if (Variables|Patrol|GetCanPatrol)
    (if (< (Transformation|GetDistanceTo self _output) (Variables|Patrol|GetPatrolAcceptanceRadius))
      (CallFunction|GetNextPatrolLocation)
      (else
        (CallFunction|DoMovementTick true true (Transformation|GetActorLocation _output))))))

(event EventBeginPlay
  (CallFunction|CheckCanPatrol)
  ;[1 1 1] Movement Tick
  (bind _returnvalue (Utilities|Time|SetTimerbyEvent (delegate Custom|MovementTic) (Variables|Movement|GetMovementTickRate) true))
  (Variables|Movement|SetMovementTimer _returnvalue)
  ;[1 1 1] Check for Player
  (bind _returnvalue_2 (Utilities|Time|SetTimerbyEvent (delegate Custom|CheckForPlayer) (Variables|CheckForPlayer|GetCheckForPlayerTick) true))
  (Variables|CheckForPlayer|SetCheckForPlayerTimer _returnvalue_2))

(fn ConstructionScript)

(fn CheckCanPatrol
  (if (> (Utilities|Array|Length (Variables|Patrol|GetPatrolPoints)) 0)
    (for _array_element (Variables|Patrol|GetPatrolPoints)
      (Utilities|IsValid _array_element
        (:Is%20Not%20Valid
          (Math|Integer|IncrementInt (LocalVariables|GetInvalidIndexes)))))
    (Variables|Patrol|SetCanPatrol (!= (LocalVariables|GetInvalidIndexes) (Utilities|Array|Length (Variables|Patrol|GetPatrolPoints))))
    (else
      (Variables|Patrol|SetCanPatrol false))))

(fn GetNextPatrolLocation
  (bind _output_get (Variables|Patrol|SetPatrolIndex (Math|Integer|SelectInt 0 (+ (Variables|Patrol|GetPatrolIndex) 1) (== (+ (Variables|Patrol|GetPatrolIndex) 1) (Utilities|Array|Length (Variables|Patrol|GetPatrolPoints)))) :!label _label))
  (Utilities|IsValid (Utilities|Array|Get(acopy) (Variables|Patrol|GetPatrolPoints) _output_get)
    (:Is%20Not%20Valid
      (goto _label))))

(fn TraceforPlayer
  (bind _returnvalue (Game|GetPlayerCharacter 0))
  (bind _returnvalue_2 (Transformation|GetActorLocation))
  (bind _arrow (Variables|Default|GetArrow))
  (bind _returnvalue_3 (Transformation|GetActorLocation _returnvalue))
  (bind _returnvalue_4 (Transformation|GetWorldLocation _arrow))
  (bind _returnvalue_5 (- _returnvalue_3 _returnvalue_2))
  (bind _returnvalue_6 (Math|Vector|Normalize _returnvalue_5))
  (if (> (Math|Vector|DotProduct (Math|Vector|GetForwardVector (Variables|Default|GetArrow)) _returnvalue_6) (Variables|CheckForPlayer|GetFindPlayerDot))
    (bind (_outhit _returnvalue_7) (Collision|LineTraceForObjects _returnvalue_4 (+ _returnvalue_4 (* _returnvalue_6 (Variables|CheckForPlayer|GetPlayerTraceDistance))) (Utilities|Array|MakeArray "ObjectTypeQuery1" "ObjectTypeQuery2" "ObjectTypeQuery3") false 0 (select (Variables|CheckForPlayer|GetTraceDebug) "ForDuration" "None")))
    (bind _asbp_player (Utilities|Casting|CastToBP_Player (Game|GetPlayerCharacter 0)))
    (if (and _returnvalue_7 (not (Variables|/Game/BP_Player/BP_Player.BP_Player_C|GetIn%20Ragdoll _asbp_player)))
      (return (.Location (Collision|BreakHitResult _outhit)) (== (Game|GetPlayerCharacter 0) (.HitActor (Collision|BreakHitResult _outhit))))
      (else
        (return "0, 0, 0" false)))
    (else
      (return "0, 0, 0" false))))