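; Eyeball enemy pawn that wanders the level and chases the player on sight, loading EnemyTestLevel when it reaches them.
; Tick and BeginPlay start AI moves to random reachable points around it, with a flag that clears after a short pause on success only.
; PawnSensing sets a seen flag, which is never cleared in practice, and FollowPlayer issues a move toward the player character.
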(event OnSeePawn(PawnSensing)
  (params (Pawn :type Pawn%20Object%20Reference))
  (Variables|Default|SetisSeeingPlayer true)
  (CallFunction|FollowPlayer))

(event Custom|FollowPlayer
  (if (Variables|Default|GetisSeeingPlayer)
    (AI|AIMoveTo self "0, 0, 0" (Game|GetPlayerCharacter 0) 1.0 false
      (:OnSuccess
        (Game|OpenLevel(byObjectReference) "/Game/Maps/EnemyTestLevel.EnemyTestLevel")))
    (else
      (Variables|Default|SetisSeeingPlayer false))))

(event EventBeginPlay
  (AI|AIMoveTo self (.RandomLocation (AI|Navigation|GetRandomReachablePointinRadius (Transformation|GetActorLocation) 5e+03 0 0)) 0 1.0 false
    (:OnSuccess
      (Utilities|FlowControl|Delay 2.0)
      (Variables|Default|SetisAIMoving false))))

(event Collision|EventActorBeginOverlap
  (params (OtherActor :type Actor%20Object%20Reference)))

(event EventTick
  (params (DeltaSeconds :type Float%20%28single-precision%29))
  (if (not (Variables|Default|GetisAIMoving))
    (Variables|Default|SetisAIMoving true)
    (AI|AIMoveTo self (.RandomLocation (AI|Navigation|GetRandomReachablePointinRadius (Transformation|GetActorLocation) 5e+03 0 0)) 0 1.0 false
      (:OnSuccess
        (Utilities|FlowControl|Delay 2.0)
        (Variables|Default|SetisAIMoving false)))))

(fn ConstructionScript)