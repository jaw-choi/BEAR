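; RagdollTrigger is a box trigger volume that makes the player character ragdoll when they enter it.
; On BeginPlay it casts player character 0 to BP_Player and caches the reference.
; Box begin overlap by that player calls Ragdoll and sets the player's InTrigger flag, and end overlap clears the flag.
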(event OnComponentBeginOverlap(Box)
  (params (OverlappedComponent :type Primitive%20Component%20Object%20Reference) (OtherActor :type Actor%20Object%20Reference) (OtherComp :type Primitive%20Component%20Object%20Reference) (OtherBodyIndex :type Integer) (bFromSweep :type Boolean) (SweepResult :type Hit%20Result%20Structure%20%28by%20ref%29))
  (if (== OtherActor (Variables|Default|Getplayer))
    (Default|Ragdoll (Variables|Default|Getplayer))
    (Variables|/Game/BP_Player/BP_Player.BP_Player_C|SetIn%20Trigger (Variables|Default|Getplayer) true)))

(event OnComponentEndOverlap(Box)
  (params (OverlappedComponent :type Primitive%20Component%20Object%20Reference) (OtherActor :type Actor%20Object%20Reference) (OtherComp :type Primitive%20Component%20Object%20Reference) (OtherBodyIndex :type Integer))
  (if (== OtherActor (Variables|Default|Getplayer))
    (Variables|/Game/BP_Player/BP_Player.BP_Player_C|SetIn%20Trigger (Variables|Default|Getplayer) false)))

(event EventBeginPlay
  (bind _asbp_player (Utilities|Casting|CastToBP_Player (Game|GetPlayerCharacter 0)))
  (Variables|Default|Setplayer _asbp_player))

(event Collision|EventActorBeginOverlap
  (params (OtherActor :type Actor%20Object%20Reference)))

(event EventTick
  (params (DeltaSeconds :type Float%20%28single-precision%29)))

(fn ConstructionScript)