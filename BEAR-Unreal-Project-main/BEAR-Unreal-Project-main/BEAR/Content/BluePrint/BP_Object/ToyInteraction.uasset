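; Interactable toy that saves the player's location as their respawn point and shows a full interaction widget from a configurable image class.
; A collision box tracks player overlap, while Tick polls the player's interaction flags.
; The first interaction locks input and reveals the widget with its fade-out animation; the next plays fade-in, hides it and restores input.
; Delays timed by the animations' return values sequence both transitions.
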(event OnComponentBeginOverlap(CollisionBox)
  (params (OverlappedComponent :type Primitive%20Component%20Object%20Reference) (OtherActor :type Actor%20Object%20Reference) (OtherComp :type Primitive%20Component%20Object%20Reference) (OtherBodyIndex :type Integer) (bFromSweep :type Boolean) (SweepResult :type Hit%20Result%20Structure%20%28by%20ref%29))
  (if (== OtherActor (Variables|Default|GetPlayer))
    (Variables|Default|SetIsColliding true)))

(event OnComponentEndOverlap(CollisionBox)
  (params (OverlappedComponent :type Primitive%20Component%20Object%20Reference) (OtherActor :type Actor%20Object%20Reference) (OtherComp :type Primitive%20Component%20Object%20Reference) (OtherBodyIndex :type Integer))
  (if (== OtherActor (Variables|Default|GetPlayer))
    (Variables|Default|SetIsColliding false)))

(event EventBeginPlay
  (bind _asbp_player (Utilities|Casting|CastToBP_Player (Game|GetPlayerCharacter 0)))
  (Variables|Default|SetPlayer _asbp_player)
  (bind _returnvalue (UserInterface|CreateWidget (Variables|Default|GetImage)))
  (bind _astoy_interaction_parent (Utilities|Casting|CastToToyInteractionParent _returnvalue))
  (bind _output_get (Variables|Default|SetToy _astoy_interaction_parent))
  (UserInterface|Viewport|AddtoViewport _output_get 0)
  (Widget|SetVisibility (Variables|Default|GetToy) "Hidden")
  (Variables|Default|SetIsInteracting false)
  (Variables|Default|SetIsColliding false))

(event Collision|EventActorBeginOverlap
  (params (OtherActor :type Actor%20Object%20Reference)))

(event EventTick
  (params (DeltaSeconds :type Float%20%28single-precision%29))
  (if (Variables|/Game/BP_Player/BP_Player.BP_Player_C|GetcanInteractWithToy (Variables|Default|GetPlayer))
    (if (not (Variables|/Game/BP_Player/BP_Player.BP_Player_C|GetIsInteractWithToy (Variables|Default|GetPlayer)))
      (if (Variables|Default|GetIsColliding)
        (Class|MainCharacter|SetPlayerRespawnPos (Variables|Default|GetPlayer) (Transformation|GetActorLocation (Variables|Default|GetPlayer)))
        (Widget|SetVisibility (Variables|Default|GetToy) "Visible")
        (Variables|/Game/BP_Player/BP_Player.BP_Player_C|SetCanGetInput (Variables|Default|GetPlayer) false)
        (Variables|/Game/BP_Player/BP_Player.BP_Player_C|SetIsInteractWithToy (Variables|Default|GetPlayer) true)
        (bind _endtime (Default|PlayFadeOut (Variables|Default|GetToy)))
        (Utilities|FlowControl|Delay _endtime)
        (Variables|Default|SetIsAnimDone true)
        (Variables|/Game/BP_Player/BP_Player.BP_Player_C|SetcanInteractWithToy (Variables|Default|GetPlayer) false))
      (elif (Variables|Default|GetIsAnimDone)
        (Variables|Default|SetIsAnimDone false)
        (bind _endtime_2 (Default|PlayFadein (Variables|Default|GetToy)))
        (Utilities|FlowControl|Delay _endtime_2)
        (Widget|SetVisibility (Variables|Default|GetToy) "Hidden")
        (Variables|/Game/BP_Player/BP_Player.BP_Player_C|SetIsInteractWithToy (Variables|Default|GetPlayer) false)
        (Variables|/Game/BP_Player/BP_Player.BP_Player_C|SetCanGetInput (Variables|Default|GetPlayer) true)
        (Variables|/Game/BP_Player/BP_Player.BP_Player_C|SetcanInteractWithToy (Variables|Default|GetPlayer) false)))))

(fn ConstructionScript)