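; Slide zone object that makes the player slide while overlapping its Box component.
; On BeginPlay it caches the player character as BP_Player.
; Box overlap begin removes ground friction, nearly removes walking braking, shrinks the walkable floor angle and sets the player's IsSliding flag.
; Overlap end restores hard-coded movement values and clears the flag; neither event checks which actor triggered it.
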(event OnComponentBeginOverlap(Box)
  (params (OverlappedComponent :type Primitive%20Component%20Object%20Reference) (OtherActor :type Actor%20Object%20Reference) (OtherComp :type Primitive%20Component%20Object%20Reference) (OtherBodyIndex :type Integer) (bFromSweep :type Boolean) (SweepResult :type Hit%20Result%20Structure%20%28by%20ref%29))
  (bind _player (Variables|Default|GetPlayer))
  (bind _charactermovement (Variables|/Script/Engine.Character|GetCharacterMovement _player))
  (Variables|/Script/Engine.CharacterMovementComponent|SetGroundFriction _charactermovement 0.0)
  (Variables|/Script/Engine.CharacterMovementComponent|SetBrakingDecelerationWalking _charactermovement 0.1)
  (Pawn|Components|CharacterMovement|SetWalkableFloorAngle _charactermovement 1.0)
  (Variables|/Game/BP_Player/BP_Player.BP_Player_C|SetIsSliding (Variables|Default|GetPlayer) true))

(event OnComponentEndOverlap(Box)
  (params (OverlappedComponent :type Primitive%20Component%20Object%20Reference) (OtherActor :type Actor%20Object%20Reference) (OtherComp :type Primitive%20Component%20Object%20Reference) (OtherBodyIndex :type Integer))
  (bind _player (Variables|Default|GetPlayer))
  (bind _charactermovement (Variables|/Script/Engine.Character|GetCharacterMovement _player))
  (Variables|/Script/Engine.CharacterMovementComponent|SetGroundFriction _charactermovement 8.0)
  (Variables|/Script/Engine.CharacterMovementComponent|SetBrakingDecelerationWalking _charactermovement 2048.0)
  (Pawn|Components|CharacterMovement|SetWalkableFloorAngle _charactermovement 45.0)
  (Variables|/Game/BP_Player/BP_Player.BP_Player_C|SetIsSliding (Variables|Default|GetPlayer) false))

(event EventBeginPlay
  (bind _asbp_player (Utilities|Casting|CastToBP_Player (Game|GetPlayerCharacter 0)))
  (Variables|Default|SetPlayer _asbp_player))

(event Collision|EventActorBeginOverlap
  (params (OtherActor :type Actor%20Object%20Reference)))

(event EventTick
  (params (DeltaSeconds :type Float%20%28single-precision%29)))

(fn ConstructionScript)