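; BP_OpenTirggerBoxWithMovableBox is a trigger Blueprint that plays a level sequence on overlap, apparently meant to open something when a movable box enters.
; On begin overlap, it plays LevelSequence1 if OtherActor equals the result of GetComponentByClass(PushComponent), comparing an actor to a component rather than checking validity.
; End overlap does nothing; the matching reverse-playback branch is disconnected and never runs.
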(event Collision|EventActorBeginOverlap
  (params (OtherActor :type Actor%20Object%20Reference))
  (if (== OtherActor (Actor|GetComponentbyClass "/Game/PushableObject/PushComponent.PushComponent_C"))
    (Sequencer|Player|Play (Variables|/Script/LevelSequence.LevelSequenceActor|GetSequencePlayer (Variables|Default|GetLevelSequence1)) :!class /Script/MovieScene.MovieSceneSequencePlayer)))

(event Collision|EventActorEndOverlap
  (params (OtherActor :type Actor%20Object%20Reference)))

(fn ConstructionScript)