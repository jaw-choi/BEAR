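; Trigger actor that transitions the player to the Employee_Area level with a short scripted walk-off.
; When BP_Player overlaps it, it plays an optional level sequence and spawns the pawn's default controller so AIMoveTo can walk it near the Destination component.
; As the move starts, the view blends to this actor and the camera fades out, then the level opens after a fixed delay without waiting for arrival.
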(event Collision|EventActorBeginOverlap
  (params (OtherActor :type Actor%20Object%20Reference))
  (bind _asbp_player (Utilities|Casting|CastToBP_Player OtherActor))
  (if (== _asbp_player OtherActor)
    (if (Utilities|IsValid (Variables|Default|GetLevelSequenceTpPlay))
      (Sequencer|Player|Play (Variables|/Script/LevelSequence.LevelSequenceActor|GetSequencePlayer (Variables|Default|GetLevelSequenceTpPlay)) :!class /Script/MovieScene.MovieSceneSequencePlayer))
    (Pawn|SpawnDefaultController _asbp_player)
    (AI|AIMoveTo _asbp_player (.RandomLocation (Class|NavigationSystemV1|GetRandomPointinNavigableRadius (Transformation|GetWorldLocation (Variables|Default|GetDestination)) 5e+01 0 0)) 0 5.0 false
      (:then
        (Game|Player|SetViewTargetwithBlend (Game|GetPlayerController 0) self 1.0 "VTBlend_Linear" 0.0 false)
        (CameraFades|StartCameraFade :self (Game|GetPlayerCameraManager 0) :ToAlpha 1.0 :Duration 1.0 :bHoldWhenFinished true)
        (Utilities|FlowControl|Delay 1.5)
        (Game|OpenLevel(byObjectReference) "/Game/Maps/Employee_Area.Employee_Area")))))

(fn ConstructionScript)