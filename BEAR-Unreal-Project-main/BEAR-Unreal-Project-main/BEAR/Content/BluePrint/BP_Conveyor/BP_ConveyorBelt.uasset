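; BP_ConveyorBelt is a conveyor belt that carries BP_Player actors along the forward direction of its Box.
; Every Tick it checks the Box's overlaps, offsetting standing players by ConveyorSpeed scaled by delta time, without sweep.
; Ragdolled players instead get a fixed mesh impulse each frame, not scaled by delta time.
; The construction script gives the Cube a dynamic material and sets its texture X scale.
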(event EventBeginPlay)

(event Collision|EventActorBeginOverlap
  (params (OtherActor :type Actor%20Object%20Reference)))

(event EventTick
  (params (DeltaSeconds :type Float%20%28single-precision%29))
  (for _array_element (Collision|GetOverlappingActors (Variables|Default|GetBox) 0 :!class /Script/Engine.PrimitiveComponent)
    (bind _asbp_player (Utilities|Casting|CastToBP_Player _array_element))
    (if (Variables|/Game/BP_Player/BP_Player.BP_Player_C|GetIn%20Ragdoll _asbp_player)
      (Physics|AddImpulseatLocation (Variables|/Script/Engine.Character|GetMesh _asbp_player) (* (Math|Vector|GetForwardVector (Transformation|GetWorldRotation (Variables|Default|GetBox))) 2.5e+02) (Transformation|GetWorldLocation (Variables|/Script/Engine.Character|GetMesh _asbp_player)) "None")
      (else
        (Transformation|AddActorWorldOffset _array_element (* (Math|Vector|GetForwardVector (Transformation|GetWorldRotation (Variables|Default|GetBox))) (* DeltaSeconds (Variables|Default|GetConveyorSpeed))))))))

(fn ConstructionScript
  (bind _cube (Variables|Default|GetCube))
  (bind _returnvalue (Rendering|Material|CreateDynamicMaterialInstance _cube 0 0 "None" :!class /Script/Engine.PrimitiveComponent))
  (Rendering|Material|SetMaterial _cube 0 _returnvalue)
  (Rendering|Material|SetScalarParameterValue _returnvalue "Texture X Scale" 5.0 :!class /Script/Engine.MaterialInstanceDynamic))