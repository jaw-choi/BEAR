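; PatrollingAI is an AI-controlled pawn Blueprint that hands its behavior tree setup to a MY_AIC controller.
; On BeginPlay it casts its controller to MY_AIC and calls SetupAIC with its BT and the first player pawn as the pawn-sensing target.
; The Construction Script creates a dynamic emissive eye material on the Sphere and passes it to GenericEmissiveColorChangingComponent for color changes.
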(event EventBeginPlay
  (bind _asmy_aic (Utilities|Casting|CastToMY_AIC (AI|GetAIController self)))
  (Default|SetupAIC _asmy_aic (Variables|Default|GetBT) (Game|Player|GetPlayerPawn 0)))

(fn ConstructionScript
  (bind _returnvalue (Rendering|Material|CreateDynamicMaterialInstance (Variables|Default|GetSphere) 0 "/Game/BluePrint/BT/Skywatcher/GenericEmissiveColour.GenericEmissiveColour" "None" :!class /Script/Engine.PrimitiveComponent))
  (bind _output_get (Variables|Default|SetDynamicEyeMatRef _returnvalue))
  (Default|Setup (Variables|Default|GetGenericEmissiveColorChangingComponent) _output_get))