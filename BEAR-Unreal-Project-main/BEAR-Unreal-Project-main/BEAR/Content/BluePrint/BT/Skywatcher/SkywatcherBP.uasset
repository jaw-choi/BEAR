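; Skywatcher is an AI-controlled actor with a colour-changing emissive eye and physics-based movement parameters.
; The construction script creates a dynamic material on the eye for GenericEmissiveColorChangingComponent to control, then initializes PhysicsMoveToParameters.
; On BeginPlay it passes its behavior tree and the player pawn, as the sensing target, to its MY_AIC controller.
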(event EventBeginPlay
  (bind _asmy_aic (Utilities|Casting|CastToMY_AIC (AI|GetAIController self)))
  (Default|SetupAIC _asmy_aic (Variables|Default|GetBT) (Game|Player|GetPlayerPawn 0)))

(fn ConstructionScript
  ;[1 1 1] Setup Dynamic Eye Material and Component
  (bind _returnvalue (Rendering|Material|CreateDynamicMaterialInstance (Variables|Default|GetEye) 0 "/Game/BluePrint/BT/Skywatcher/GenericEmissiveColour.GenericEmissiveColour" "None" :!class /Script/Engine.PrimitiveComponent))
  (bind _output_get (LocalVariables|SetDynamicEyeMatRef _returnvalue))
  (Default|Setup (Variables|Default|GetGenericEmissiveColorChangingComponent) _output_get)
  ;[1 1 1] Setup Physics
  (Default|Setup (Variables|Default|GetPhysicsMoveToParameters)))