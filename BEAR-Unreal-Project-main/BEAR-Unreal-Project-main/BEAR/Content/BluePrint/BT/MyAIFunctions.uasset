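; MyAIFunctions is a set of shared helper functions for AI Blueprints, covering Blackboard writes and component lookup.
; UpdateBBKey switches on a key type to write a Bool, Actor, Vector or Rotator value to the AI controller's Blackboard under the given key name.
; GetComponentIFValid fetches a component by class from an owner, returning a validity flag with the reference, or printing a debug message when the lookup fails.
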(fn UpdateBBKey
  (params (AIController :type AI%20Controller%20Object%20Reference) (KeyName :type Name) (KeyType :type KeyTypes%20Enum :default "NewEnumerator0") (BoolValue :type Boolean) (ObjectValue :type Object%20Object%20Reference) (VectorValue :type Vector) (RotatorValue :type Rotator))
  (bind _returnvalue (Utilities|Name|MakeLiteralName KeyName))
  (bind _returnvalue_2 (AI|GetBlackboard AIController))
  (switch Utilities|FlowControl|Switch|SwitchonKeyTypes KeyType
    (:NewEnumerator0
      (AI|Components|Blackboard|SetValueasBool _returnvalue_2 _returnvalue BoolValue))
    (:NewEnumerator1
      (AI|Components|Blackboard|SetValueasObject _returnvalue_2 _returnvalue ObjectValue))
    (:NewEnumerator2
      (AI|Components|Blackboard|SetValueasVector _returnvalue_2 _returnvalue VectorValue))
    (:NewEnumerator3
      (Class|BlackboardComponent|SetValueasRotator _returnvalue_2 _returnvalue RotatorValue))))

(fn GetComponentIFValid
  (params (Owner :type Actor%20Object%20Reference) (ComponentClass :type Actor%20Component%20Class%20Reference))
  (bind _returnvalue (Actor|GetComponentbyClass Owner ComponentClass))
  (Utilities|IsValid _returnvalue
    (:Is%20Valid
      (return true _returnvalue))
    (:Is%20Not%20Valid
      (Development|PrintString 0 (Utilities|String|Append "Tried to get component but wasn't valid" (Utilities|GetDisplayName _returnvalue) "Owner" (Utilities|GetDisplayName Owner)))
      (return false 0))))