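; BP_Pushable_V2 is a pushable crate that becomes physics-driven when the player touches its trigger volumes.
; Separate X-axis and Y-axis collision components filter overlaps to BP_Player and enable physics simulation on Crate1.
; Both begin and end overlap set simulation to true, so nothing in the graph turns physics back off.
; Neither axis applies any movement constraint here, and both behave identically.
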(event OnComponentBeginOverlap(XAxisCollision)
  (params (OverlappedComponent :type Primitive%20Component%20Object%20Reference) (OtherActor :type Actor%20Object%20Reference) (OtherComp :type Primitive%20Component%20Object%20Reference) (OtherBodyIndex :type Integer) (bFromSweep :type Boolean) (SweepResult :type Hit%20Result%20Structure%20%28by%20ref%29))
  ;[1 1 1] X Axis Collision
  (Utilities|Casting|CastToBP_Player OtherActor)
  (Physics|SetSimulatePhysics (Variables|Default|GetCrate1) true))

(event OnComponentEndOverlap(XAxisCollision)
  (params (OverlappedComponent :type Primitive%20Component%20Object%20Reference) (OtherActor :type Actor%20Object%20Reference) (OtherComp :type Primitive%20Component%20Object%20Reference) (OtherBodyIndex :type Integer))
  ;[1 1 1] X Axis Collision
  (Utilities|Casting|CastToBP_Player OtherActor)
  (Physics|SetSimulatePhysics (Variables|Default|GetCrate1) true))

(event OnComponentBeginOverlap(YAxisCollision)
  (params (OverlappedComponent :type Primitive%20Component%20Object%20Reference) (OtherActor :type Actor%20Object%20Reference) (OtherComp :type Primitive%20Component%20Object%20Reference) (OtherBodyIndex :type Integer) (bFromSweep :type Boolean) (SweepResult :type Hit%20Result%20Structure%20%28by%20ref%29))
  ;[1 1 1] Y Axis collision
  (Utilities|Casting|CastToBP_Player OtherActor)
  (Physics|SetSimulatePhysics (Variables|Default|GetCrate1) true))

(event OnComponentEndOverlap(YAxisCollision)
  (params (OverlappedComponent :type Primitive%20Component%20Object%20Reference) (OtherActor :type Actor%20Object%20Reference) (OtherComp :type Primitive%20Component%20Object%20Reference) (OtherBodyIndex :type Integer))
  ;[1 1 1] Y Axis collision
  (Utilities|Casting|CastToBP_Player OtherActor)
  (Physics|SetSimulatePhysics (Variables|Default|GetCrate1) true))

(event EventBeginPlay)

(event EventTick
  (params (DeltaSeconds :type Float%20%28single-precision%29)))

(fn ConstructionScript)